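; Non-Euclidean magic window that shows or hides its assigned MagicActors depending on which side of it the player's camera is.
; While a Character overlaps the Plane, Tick tests the player's CamTracker child points against the Arrow's normal via FLIsPlayerFront.
; Any point in front calls Visible on each actor's AC_MagicComp; otherwise NotVisible.
; Construction sets the Plane's custom depth stencil from StencilFilter; the local plane-crossing function IsPlayerFront is uncalled.
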(event `self.ReceiveBeginPlay`
  (bind _asbp_first_person_character (cast `/Game/NonEuclideanTemplate/Blueprints/Core/FirstPerson/Blueprints/BP_FirstPersonCharacter` (`GameplayStatics.GetPlayerPawn` 0))
    (:`then`
      (set `self.Cam Tracker` (`/Game/NonEuclideanTemplate/Blueprints/Core/FirstPerson/Blueprints/BP_FirstPersonCharacter.CamTracker` _asbp_first_person_character)))
    (:`CastFailed`
      (`KismetSystemLibrary.PrintString` "Debug - MagicWindow - No First Person"))))

(event `self.Plane.OnComponentBeginOverlap`
  (params (OverlappedComponent :type "PrimitiveComponent Object Reference") (OtherActor :type "Actor Object Reference") (OtherComp :type "PrimitiveComponent Object Reference") (OtherBodyIndex :type Integer) (bFromSweep :type Boolean) (SweepResult :type "HitResult Structure (by ref)"))
  (cast `Character` OtherActor)
  (set `self.OverlappingPlayer` true))

(event `self.ReceiveTick`
  (params (DeltaSeconds :type "Float (single-precision)"))
  (if (`self.OverlappingPlayer`)
    (set `self.ShowObjects` false)
    (for _array_element (`SceneComponent.GetChildrenComponents` (`self.Cam Tracker`) false)
      (bind _front (`/Game/NonEuclideanTemplate/Blueprints/NonEuclidian/FL_lib.FL_IsPlayerFront` (`SceneComponent.K2_GetComponentLocation` _array_element) (`self.K2_GetActorLocation`) (`SceneComponent.GetForwardVector` (`self.Arrow`))))
      (set `self.ShowObjects` _front)
      (if (`self.ShowObjects`)
        (break)))
    (if (`self.ShowObjects`)
      (for _array_element_2 (`self.MagicActors`)
        (`/Engine/EditorBlueprintResources/StandardMacros.IsValid` _array_element_2
          (:`Is Valid`
            (bind _returnvalue (`self.GetComponentByClass` _array_element_2 "/Game/NonEuclideanTemplate/Blueprints/NonEuclidian/AC_MagicComp.AC_MagicComp_C"))
            (`/Engine/EditorBlueprintResources/StandardMacros.IsValid` _returnvalue
              (:`Is Valid`
                (`/Game/NonEuclideanTemplate/Blueprints/NonEuclidian/AC_MagicComp.Visible` _returnvalue))))))
      (else
        (for _array_element_3 (`self.MagicActors`)
          (`/Engine/EditorBlueprintResources/StandardMacros.IsValid` _array_element_3
            (:`Is Valid`
              (bind _returnvalue_2 (`self.GetComponentByClass` _array_element_3 "/Game/NonEuclideanTemplate/Blueprints/NonEuclidian/AC_MagicComp.AC_MagicComp_C"))
              (`/Engine/EditorBlueprintResources/StandardMacros.IsValid` _returnvalue_2
                (:`Is Valid`
                  (`/Game/NonEuclideanTemplate/Blueprints/NonEuclidian/AC_MagicComp.NotVisible` _returnvalue_2))))))))))

(event `self.Plane.OnComponentEndOverlap`
  (params (OverlappedComponent :type "PrimitiveComponent Object Reference") (OtherActor :type "Actor Object Reference") (OtherComp :type "PrimitiveComponent Object Reference") (OtherBodyIndex :type Integer))
  (cast `Character` OtherActor)
  (set `self.OverlappingPlayer` false))

(fn `IsPlayerFront`
  (params (PlayerCam :type "Vector Structure") (WindowLocation :type "Vector Structure") (WindowNormal :type "Vector Structure"))
  (returns (Return :type Boolean))
  (set `self.IsFront` (>= (`KismetMathLibrary.Dot_VectorVector` (- PlayerCam WindowLocation) WindowNormal) 0.0))
  (set `self.Intersect` (`.ReturnValue` (`KismetMathLibrary.LinePlaneIntersection` (`self.LastLocation`) PlayerCam (`KismetMathLibrary.MakePlaneFromPointAndNormal` WindowLocation WindowNormal))))
  (set `self.IsCrossing` (and (`self.Intersect`) (not (`self.IsFront`))))
  (set `self.LastLocation` PlayerCam)
  (return (`self.IsCrossing`)))

(fn `UserConstructionScript`
  (`PrimitiveComponent.SetCustomDepthStencilValue` (`self.Plane`) (`self.StencilFilter`)))
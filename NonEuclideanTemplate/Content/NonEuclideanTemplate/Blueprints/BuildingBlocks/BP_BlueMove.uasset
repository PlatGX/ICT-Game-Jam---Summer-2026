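; BP_BlueMove is a moving block actor that shuttles its Cube back and forth between Start and End points.
; BeginPlay teleports the Cube to Start, then Tick accumulates time in the current direction and lerps its position over Duration.
; Passing either end toggles a gate to pause movement, waits for Delay, flips the direction and reopens the gate.
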(event `self.ReceiveBeginPlay`
  (`SceneComponent.K2_SetWorldLocation` (`self.Cube`) (`SceneComponent.K2_GetComponentLocation` (`self.Start`)) false true))

(event `self.ReceiveTick`
  (params (DeltaSeconds :type "Float (single-precision)"))
  (bind _returnvalue (/ (`self.Alpha`) (`self.Duration`)))
  (`/Engine/EditorBlueprintResources/StandardMacros.Gate` false :!label _label
    (:`Exit`
      (set `self.Alpha` (+ (* DeltaSeconds (`self.Dir`)) (`self.Alpha`)))
      (`SceneComponent.K2_SetWorldLocation` (`self.Cube`) (`KismetMathLibrary.VLerp` (`SceneComponent.K2_GetComponentLocation` (`self.Start`)) (`SceneComponent.K2_GetComponentLocation` (`self.End`)) (/ (`self.Alpha`) (`self.Duration`))) false false)
      (if (or (< _returnvalue 0.0) (> _returnvalue 1.0))
        (`self.ToggleGate`)
        (`KismetSystemLibrary.Delay` (`self.Delay`))
        (set `self.Dir` (* (`self.Dir`) -1.0))
        (`self.ToggleGate`)))))

(event `ToggleGate`
  (goto _label :!via `Toggle`))

(fn `UserConstructionScript`)
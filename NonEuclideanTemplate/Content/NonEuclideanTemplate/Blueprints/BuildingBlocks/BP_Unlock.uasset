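; BP_Unlock is a pickup actor that unlocks one of three R, G or B flags when the player touches it.
; A sphere overlap with the player character uses the RGB value to select which flag to set on the GI_Unlocks game instance.
; After setting the flag, it waits through a zero-length delay and destroys itself.
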(event `self.Sphere.OnComponentBeginOverlap`
  (params (OverlappedComponent :type "PrimitiveComponent Object Reference") (OtherActor :type "Actor Object Reference") (OtherComp :type "PrimitiveComponent Object Reference") (OtherBodyIndex :type Integer) (bFromSweep :type Boolean) (SweepResult :type "HitResult Structure (by ref)"))
  (if (== OtherActor (`GameplayStatics.GetPlayerCharacter` 0))
    (bind _asgi_unlocks (cast `/Game/NonEuclideanTemplate/Blueprints/Core/FirstPerson/Blueprints/GI_Unlocks` (`GameplayStatics.GetGameInstance`)))
    (switch `int` (`self.RGB?`)
      (:`1`
        (set `/Game/NonEuclideanTemplate/Blueprints/Core/FirstPerson/Blueprints/GI_Unlocks.UnlockedR` true _asgi_unlocks))
      (:`2`
        (set `/Game/NonEuclideanTemplate/Blueprints/Core/FirstPerson/Blueprints/GI_Unlocks.UnlockedG` true _asgi_unlocks))
      (:`3`
        (set `/Game/NonEuclideanTemplate/Blueprints/Core/FirstPerson/Blueprints/GI_Unlocks.UnlockedB` true _asgi_unlocks)))
    (`KismetSystemLibrary.Delay` 0.0)
    (`self.K2_DestroyActor`)))

(fn `UserConstructionScript`)
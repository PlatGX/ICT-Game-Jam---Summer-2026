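; Actor component that toggles its owner between hidden, non-colliding and visible, solid states, starting hidden on BeginPlay when Enabled.
; NotVisible and Visible set a "Visible" scalar on new dynamic material instances for every static and skeletal mesh material.
; Static meshes also switch between NoCollision and BlockAll, with physics simulation toggled where a helper function allows it.
; Character owners also switch their capsule between NoCollision and Pawn.
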(event `self.ReceiveBeginPlay`
  (if (`self.Enabled`)
    (`self.NotVisible`)))

(event `NotVisible`
  (bind _returnvalue (`self.GetOwner`))
  ;[1 1 1] No visibility no collision
  (for _array_element (`Actor.K2_GetComponentsByClass` _returnvalue "/Script/Engine.StaticMeshComponent")
    (`/Engine/EditorBlueprintResources/StandardMacros.IsValid` _array_element
      (:`Is Valid`
        (bind _startedwithsimulatephysic (`/Game/NonEuclideanTemplate/Blueprints/FL_lib.FL_ShouldSimulatePhysic` _array_element))
        (if _startedwithsimulatephysic
          (`PrimitiveComponent.SetSimulatePhysics` _array_element false))
        (`PrimitiveComponent.SetCollisionProfileName` _array_element "NoCollision" true)
        (for _index (range (`PrimitiveComponent.GetNumMaterials` _array_element))
          (bind _output (`|GetArrayItem` (`MeshComponent.GetMaterials` _array_element) _index))
          (`/Engine/EditorBlueprintResources/StandardMacros.IsValid` _output
            (:`Is Valid`
              (bind _returnvalue_2 (`PrimitiveComponent.CreateDynamicMaterialInstance` _array_element _index _output "None"))
              (`PrimitiveComponent.SetMaterial` _array_element _index _returnvalue_2)
              (`MaterialInstanceDynamic.SetScalarParameterValue` _returnvalue_2 "Visible" 0.0)))))))
  (for _array_element_2 (`Actor.K2_GetComponentsByClass` _returnvalue "/Script/Engine.SkeletalMeshComponent")
    (`/Engine/EditorBlueprintResources/StandardMacros.IsValid` _array_element_2
      (:`Is Valid`
        (for _index_2 (range (`PrimitiveComponent.GetNumMaterials` _array_element_2))
          (bind _output_2 (`|GetArrayItem` (`MeshComponent.GetMaterials` _array_element_2) _index_2))
          (`/Engine/EditorBlueprintResources/StandardMacros.IsValid` _output_2
            (:`Is Valid`
              (bind _returnvalue_3 (`PrimitiveComponent.CreateDynamicMaterialInstance` _array_element_2 _index_2 _output_2 "None"))
              (`PrimitiveComponent.SetMaterial` _array_element_2 _index_2 _returnvalue_3)
              (`MaterialInstanceDynamic.SetScalarParameterValue` _returnvalue_3 "Visible" 0.0)))))))
  (bind _ascharacter (cast `Character` _returnvalue))
  (`PrimitiveComponent.SetCollisionProfileName` (`Character.CapsuleComponent` _ascharacter) "NoCollision" true))

(event `Visible`
  (bind _returnvalue (`self.GetOwner`))
  ;[1 1 1] visbility and colision enabled
  (for _array_element (`Actor.K2_GetComponentsByClass` _returnvalue "/Script/Engine.StaticMeshComponent")
    (`/Engine/EditorBlueprintResources/StandardMacros.IsValid` _array_element
      (:`Is Valid`
        (bind _startedwithsimulatephysic (`/Game/NonEuclideanTemplate/Blueprints/FL_lib.FL_ShouldSimulatePhysic` _array_element))
        (if _startedwithsimulatephysic
          (`PrimitiveComponent.SetSimulatePhysics` _array_element true))
        (`PrimitiveComponent.SetCollisionProfileName` _array_element "BlockAll" true)
        (for _index (range (`PrimitiveComponent.GetNumMaterials` _array_element))
          (bind _output (`|GetArrayItem` (`MeshComponent.GetMaterials` _array_element) _index))
          (`/Engine/EditorBlueprintResources/StandardMacros.IsValid` _output
            (:`Is Valid`
              (bind _returnvalue_2 (`PrimitiveComponent.CreateDynamicMaterialInstance` _array_element _index _output "None"))
              (`PrimitiveComponent.SetMaterial` _array_element _index _returnvalue_2)
              (`MaterialInstanceDynamic.SetScalarParameterValue` _returnvalue_2 "Visible" 1.0)))))))
  (for _array_element_2 (`Actor.K2_GetComponentsByClass` _returnvalue "/Script/Engine.SkeletalMeshComponent")
    (`/Engine/EditorBlueprintResources/StandardMacros.IsValid` _array_element_2
      (:`Is Valid`
        (for _index_2 (range (`PrimitiveComponent.GetNumMaterials` _array_element_2))
          (bind _output_2 (`|GetArrayItem` (`MeshComponent.GetMaterials` _array_element_2) _index_2))
          (`/Engine/EditorBlueprintResources/StandardMacros.IsValid` _output_2
            (:`Is Valid`
              (bind _returnvalue_3 (`PrimitiveComponent.CreateDynamicMaterialInstance` _array_element_2 _index_2 _output_2 "None"))
              (`PrimitiveComponent.SetMaterial` _array_element_2 _index_2 _returnvalue_3)
              (`MaterialInstanceDynamic.SetScalarParameterValue` _returnvalue_3 "Visible" 1.0)))))))
  (bind _ascharacter (cast `Character` _returnvalue))
  (`PrimitiveComponent.SetCollisionProfileName` (`Character.CapsuleComponent` _ascharacter) "Pawn" true))
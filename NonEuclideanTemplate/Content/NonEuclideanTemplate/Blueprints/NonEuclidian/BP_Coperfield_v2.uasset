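; Non-Euclidean threshold module that swaps sets of level actors as the first-person player crosses its plane.
; While a character overlaps the plane, Tick tests the player camera against the arrow's normal.
; The front side shows, hides and destroys listed actors, optionally destroying itself; the other side reverses show/hide if ReturnBoxOn.
; Swaps also switch static mesh collision profiles between BlockAll and NoCollision, toggling physics where applicable.
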(event `self.ReceiveBeginPlay`
  (bind _asbp_first_person_character (cast `/Game/NonEuclideanTemplate/Blueprints/Core/FirstPerson/Blueprints/BP_FirstPersonCharacter` (`GameplayStatics.GetPlayerPawn` 0))
    (:`then`
      (set `self.Cam Tracker` (`/Game/NonEuclideanTemplate/Blueprints/Core/FirstPerson/Blueprints/BP_FirstPersonCharacter.CamTracker` _asbp_first_person_character)))
    (:`CastFailed`
      (`KismetSystemLibrary.PrintString` "Debug - MagicWindow - No First Person"))))

(event `self.ReceiveTick`
  (params (DeltaSeconds :type "Float (single-precision)"))
  (if (`self.OverlappingPlayer`)
    ;[1 1 1] Check if the player is front to this module
    (bind _front (`/Game/NonEuclideanTemplate/Blueprints/NonEuclidian/FL_lib.FL_IsPlayerFront` (`SceneComponent.K2_GetComponentLocation` (`self.Cam Tracker`)) (`SceneComponent.K2_GetComponentLocation` (`self.Plane`)) (`SceneComponent.GetForwardVector` (`self.Arrow`))))
    (if _front
      (`self.OneWay`)
      (else
        (`self.Return`)))))

(event `self.Plane.OnComponentBeginOverlap`
  (params (OverlappedComponent :type "PrimitiveComponent Object Reference") (OtherActor :type "Actor Object Reference") (OtherComp :type "PrimitiveComponent Object Reference") (OtherBodyIndex :type Integer) (bFromSweep :type Boolean) (SweepResult :type "HitResult Structure (by ref)"))
  (cast `Character` OtherActor)
  (set `self.OverlappingPlayer` true))

(event `self.Plane.OnComponentEndOverlap`
  (params (OverlappedComponent :type "PrimitiveComponent Object Reference") (OtherActor :type "Actor Object Reference") (OtherComp :type "PrimitiveComponent Object Reference") (OtherBodyIndex :type Integer))
  (cast `Character` OtherActor)
  (set `self.OverlappingPlayer` false))

(event `OneWay`
  ;[1 1 1] Hide, show and destroy all actors that need to be while the player is crossing the module One Way. This will also deal with colisions
  (for _array_element (`self.ShowActors`)
    (`/Engine/EditorBlueprintResources/StandardMacros.IsValid` _array_element
      (:`Is Valid`
        (`self.SetActorHiddenInGame` _array_element false)
        (for _array_element_2 (`self.K2_GetComponentsByClass` _array_element "/Script/Engine.StaticMeshComponent")
          (`/Engine/EditorBlueprintResources/StandardMacros.IsValid` _array_element_2
            (:`Is Valid`
              ;;[1 1 1] We need this to know if we have to deal with physic simulation
              (bind _startedwithsimulatephysic (`/Game/NonEuclideanTemplate/Blueprints/NonEuclidian/FL_lib.FL_ShouldSimulatePhysic` _array_element_2))
              (if _startedwithsimulatephysic
                (`PrimitiveComponent.SetSimulatePhysics` _array_element_2 true))
              (`PrimitiveComponent.SetCollisionProfileName` _array_element_2 "BlockAll" true)))))))
  (for _array_element_3 (`self.HideActors`)
    (`/Engine/EditorBlueprintResources/StandardMacros.IsValid` _array_element_3
      (:`Is Valid`
        (`self.SetActorHiddenInGame` _array_element_3 true)
        (for _array_element_4 (`self.K2_GetComponentsByClass` _array_element_3 "/Script/Engine.StaticMeshComponent")
          (`/Engine/EditorBlueprintResources/StandardMacros.IsValid` _array_element_4
            (:`Is Valid`
              ;;[1 1 1] We need this to know if we have to deal with physic simulation
              (bind _startedwithsimulatephysic_2 (`/Game/NonEuclideanTemplate/Blueprints/NonEuclidian/FL_lib.FL_ShouldSimulatePhysic` _array_element_4))
              (if _startedwithsimulatephysic_2
                (`PrimitiveComponent.SetSimulatePhysics` _array_element_4 false))
              (`PrimitiveComponent.SetCollisionProfileName` _array_element_4 "NoCollision" true)))))))
  (for _array_element_5 (`self.DestroyActors`)
    (`/Engine/EditorBlueprintResources/StandardMacros.IsValid` _array_element_5
      (:`Is Valid`
        (`self.K2_DestroyActor` _array_element_5))))
  (if (`self.AutoDestroy`)
    (`self.K2_DestroyActor`)))

(event `Return`
  ;[1 1 1] Hide, show and destroy all actors that need to be during return. This will also deal with colisions
  (if (`self.ReturnBoxOn`)
    (for _array_element (`self.HideActors`)
      (`/Engine/EditorBlueprintResources/StandardMacros.IsValid` _array_element
        (:`Is Valid`
          (`self.SetActorHiddenInGame` _array_element false)
          (for _array_element_2 (`self.K2_GetComponentsByClass` _array_element "/Script/Engine.StaticMeshComponent")
            (`/Engine/EditorBlueprintResources/StandardMacros.IsValid` _array_element_2
              (:`Is Valid`
                ;;[1 1 1] We need this to know if we have to deal with physic simulation
                (bind _startedwithsimulatephysic (`/Game/NonEuclideanTemplate/Blueprints/NonEuclidian/FL_lib.FL_ShouldSimulatePhysic` _array_element_2))
                (if _startedwithsimulatephysic
                  (`PrimitiveComponent.SetSimulatePhysics` _array_element_2 true))
                (`PrimitiveComponent.SetCollisionProfileName` _array_element_2 "BlockAll" true)))))))
    (for _array_element_3 (`self.ShowActors`)
      (`/Engine/EditorBlueprintResources/StandardMacros.IsValid` _array_element_3
        (:`Is Valid`
          (`self.SetActorHiddenInGame` _array_element_3 true)
          (for _array_element_4 (`self.K2_GetComponentsByClass` _array_element_3 "/Script/Engine.StaticMeshComponent")
            (`/Engine/EditorBlueprintResources/StandardMacros.IsValid` _array_element_4
              (:`Is Valid`
                ;;[1 1 1] We need this to know if we have to deal with physic simulation
                (bind _startedwithsimulatephysic_2 (`/Game/NonEuclideanTemplate/Blueprints/NonEuclidian/FL_lib.FL_ShouldSimulatePhysic` _array_element_4))
                (if _startedwithsimulatephysic_2
                  (`PrimitiveComponent.SetSimulatePhysics` _array_element_4 false))
                (`PrimitiveComponent.SetCollisionProfileName` _array_element_4 "NoCollision" true)))))))))

(fn `UserConstructionScript`)
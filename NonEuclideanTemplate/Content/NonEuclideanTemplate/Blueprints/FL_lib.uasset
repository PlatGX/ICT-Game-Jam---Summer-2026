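; FL_lib is a helper library for the non-Euclidean template, with a window side test and a physics check.
; FLIsPlayerFront uses a dot product against the window normal to tell whether the player camera is on or in front of the window plane.
; FLShouldSimulatePhysic tags a simulating static mesh component with MagicPhysic, so it still returns true for that component after simulation is switched off.
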(fn `FL_IsPlayerFront`
  (params (PlayerCam :type "Vector Structure") (WindowLocation :type "Vector Structure") (WindowNormal :type "Vector Structure"))
  (returns (Front :type Boolean))
  (locals (IsFront :type Boolean) (Intersect :type Boolean) (IsCrossing :type Boolean) (LastLocation :type "Vector Structure") (NewLocalVar :type "Vector Structure"))
  ;[0.03569 0.07108 1] is crossing?
  (return (>= (`KismetMathLibrary.Dot_VectorVector` (- PlayerCam WindowLocation) WindowNormal) 0.0)))

(fn `FL_ShouldSimulatePhysic`
  (params (StaticMeshComponent :type "StaticMeshComponent Object Reference"))
  (returns (StartedWithSimulatePhysic :type Boolean))
  (bind _returnvalue (`ActorComponent.ComponentHasTag` StaticMeshComponent "MagicPhysic"))
  ;[1 1 1] This help us to know if we should deal with the physic simulation
  (if (`SceneComponent.IsSimulatingPhysics` StaticMeshComponent "None")
    (if (not _returnvalue)
      (`KismetArrayLibrary.Array_Add` (`ActorComponent.ComponentTags` StaticMeshComponent) "MagicPhysic"))
    (elif _returnvalue
      _
      (else
        (return false))))
  (return true))
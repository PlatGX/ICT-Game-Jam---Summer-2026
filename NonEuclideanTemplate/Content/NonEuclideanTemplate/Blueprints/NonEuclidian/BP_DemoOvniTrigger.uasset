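; BP_DemoOvniTrigger is a demo trigger that sends a UFO flying off when the first-person character overlaps it.
; At BeginPlay it finds the actor tagged "OVNI" and, if RandomAppears is set, randomly destroys it so it only sometimes appears.
; Overlap enables a Tick-driven flight using randomized lerped offsets and a slight roll.
; After a short delay it destroys the UFO, then itself.
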(event `self.ReceiveBeginPlay`
  (bind _outactors (`GameplayStatics.GetAllActorsWithTag` "OVNI"))
  (bind _output (`|GetArrayItem` _outactors))
  (`/Engine/EditorBlueprintResources/StandardMacros.IsValid` _output
    (:`Is Valid`
      (bind _output_get (set `self.OVNI` _output))
      (set `self.InitLocation` (`self.K2_GetActorLocation` _output_get))
      (if (`self.RandomAppears`)
        ;[1 1 1] Make it appears only sometimes
        (if (`KismetMathLibrary.RandomBool`)
          (`self.K2_DestroyActor` (`self.OVNI`)))))))

(event `self.ReceiveActorBeginOverlap`
  (params (OtherActor :type "Actor Object Reference"))
  (bind _ovni (`self.OVNI`))
  (cast `/Game/NonEuclideanTemplate/Blueprints/Core/FirstPerson/Blueprints/BP_FirstPersonCharacter` OtherActor)
  (`/Engine/EditorBlueprintResources/StandardMacros.IsValid` _ovni
    (:`Is Valid`
      (set `self.ActivateOvni` true)
      (`KismetSystemLibrary.Delay` 5.0)
      (set `self.ActivateOvni` false)
      (`self.K2_DestroyActor` _ovni)
      (`KismetSystemLibrary.Delay` 0.2)
      (`self.K2_DestroyActor`))))

(event `self.ReceiveTick`
  (params (DeltaSeconds :type "Float (single-precision)"))
  (bind _ovni (`self.OVNI`))
  (bind _returnvalue (`self.K2_GetActorLocation` _ovni))
  (bind _returnvalue_2 (`self.K2_GetActorRotation` _ovni))
  (if (`self.ActivateOvni`)
    (`self.K2_SetActorLocation` _ovni (`KismetMathLibrary.VLerp` _returnvalue (+ _returnvalue (`KismetMathLibrary.MakeVector` (`KismetMathLibrary.RandomFloatInRange` 500.0 800.0) (`KismetMathLibrary.RandomFloatInRange` 0.0 -200.0) (`KismetMathLibrary.RandomFloatInRange` 50.0 -50.0))) 0.3) false false)
    (`self.K2_SetActorRotation` _ovni (`KismetMathLibrary.RLerp` _returnvalue_2 (`KismetMathLibrary.MakeRotator` (+ (.roll _returnvalue_2) 0.1)) 0.5) false)))

(fn `UserConstructionScript`)